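; Lobby actor that animates the brightness of the camper and killer point lights to make them blink.
; On BeginPlay, once both light references are valid, it plays a timeline whose Brightness track drives both intensities.
; Each light scales and offsets the shared value differently, so they pulse in sync over separate ranges and never drop to zero while the track stays non-negative.
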(event EventBeginPlay
  (Utilities|IsValid (Variables|Default|GetCamper_PointLight)
    (:Is%20Valid
      (Utilities|IsValid (Variables|Default|GetKiller_PointLight)
        (:Is%20Valid
          (bind _brightness (Timeline|Timeline_0 Play)
            (:Update
              (Rendering|Components|Light|SetIntensity (Variables|Default|GetCamper_PointLight) (+ (* _brightness 5e+02) 2e+02))
              (Rendering|Components|Light|SetIntensity (Variables|Default|GetKiller_PointLight) (+ (* _brightness 4e+02) 3e+02)))))))))

(fn ConstructionScript)